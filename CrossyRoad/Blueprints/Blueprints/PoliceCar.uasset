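; PoliceCar is a moving vehicle actor that drives along its local Y axis and despawns when its lifetime runs out.
; Tick moves it by MoveSpeed each frame, while a Delay throttles the LifeTotal countdown to roughly once a second, and MoveTruck destroys it at zero.
; SpawnAtLocation spawns another PoliceCar, setting its speed and returning it only for forward movement.
; ToggleDirection sets a signed speed but is not called here.
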(event EventTick
  (params (DeltaSeconds :type Float%20%28single-precision%29))
  ;[1 1 1] Despawn truck if it doesnt collide with a collision after a certain amount of time
  (CallFunction|MoveTruck)
  (Utilities|FlowControl|Delay 1.0)
  (CallFunction|DecrementLifeTotal))

(fn ConstructionScript)

(fn SpawnatLocation
  (params (SpawnPosition :type Vector) (wantsToGoForward :type Boolean) (SpawnRotation :type Rotator))
  (bind _returnvalue (Game|SpawnActorfromClass "PoliceCar_C" (Math|Transform|MakeTransform SpawnPosition SpawnRotation "1,1,1") "Undefined" 0 true 20 0))
  (bind _output_get (Variables|Default|SetisMovingForward wantsToGoForward))
  (if _output_get
    (Variables|PoliceCar_C|SetMoveSpeed _returnvalue 15.0)
    (return _returnvalue)))

(fn ToggleDirection
  (params (isMovingForward :type Boolean))
  (if isMovingForward
    (Variables|Default|SetMoveSpeed -1e+01)
    (else
      (Variables|Default|SetMoveSpeed 1e+01))))

(fn MoveTruck
  (Class|Actor|AddActorLocalTransform (Math|Transform|MakeTransform (Math|Vector|MakeVector 0.0 (Variables|Default|GetMoveSpeed) 0.0) "0, 0, 0" "1,1,1") false false)
  (if (== 0 (Variables|Default|GetlifeTotal))
    (Actor|DestroyActor)))

(fn DecrementLifeTotal
  (Variables|Default|SetlifeTotal (- (Variables|Default|GetlifeTotal) 1)))