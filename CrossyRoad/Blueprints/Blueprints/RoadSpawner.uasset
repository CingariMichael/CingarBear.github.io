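; RoadSpawner lays out the initial strip of lanes for a Crossy Road-style game when play begins.
; BeginPlay loops over the initial road count, calling SpawnRoadAtSpawnPoint, stepping Y by a fixed offset and randomly picking each following lane's facing and matching X start.
; The spawn function has branches for Road and WaterRoad, but its condition is fixed false, so only WaterRoad spawns despite the random-choice comment.
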(event EventBeginPlay
  (for _index (range 1 (Variables|Default|GetnumInitialRoads))
    ;[0.05237 0.1051 1] Randomly spawn a Road or Water Road
    (bind (_returnroad _returnwaterroad) (CallFunction|SpawnRoadatSpawnPoint (Math|Vector|MakeVector (Variables|Default|GetroadXPosition) (Variables|Default|GetRoadYPosition) (Variables|Default|GetRoadZPosition)) (Variables|Default|GetroadRotation) (Variables|Default|GetroadScale)))
    (Variables|Default|SetNewestRoad _returnroad)
    (Variables|Default|SetnewestWaterRoad _returnwaterroad)
    ;[1 0 0] Offset spawn location - Y Position
    (Variables|Default|SetRoadYPosition (+ (Variables|Default|GetRoadYPosition) (Variables|Default|GetRoadOffset)))
    (if (< (Math|Random|RandomIntegerinRange 0 5) 2)
      (Variables|Default|SetroadRotation (Math|Rotator|MakeRotator 0.0 0.0 -9e+01))
      (Variables|Default|SetroadXPosition 7.56e+03)
      (else
        (Variables|Default|SetroadRotation (Math|Rotator|MakeRotator 0.0 0.0 9e+01))
        (Variables|Default|SetroadXPosition 0.0)))))

(fn ConstructionScript)

(fn SpawnRoadatSpawnPoint
  (params (SpawnLocation :type Vector) (SpawnRotation :type Rotator) (SpawnScale :type Vector))
  (LocalVariables|SetLocalSpawnLocation SpawnLocation)
  (LocalVariables|SetLocalSpawnRotation SpawnRotation)
  (LocalVariables|SetLocalSpawnScale SpawnScale)
  (if false
    (bind _returnvalue (Game|SpawnActorfromClass "/Game/Blueprints/Road.Road_C" (Math|Transform|MakeTransform (LocalVariables|GetLocalSpawnLocation) (LocalVariables|GetLocalSpawnRotation) (LocalVariables|GetLocalSpawnScale)) "Undefined" 0 0))
    (else
      (bind _returnvalue_2 (Game|SpawnActorfromClass "/Game/Blueprints/WaterRoad.WaterRoad_C" (Math|Transform|MakeTransform (LocalVariables|GetLocalSpawnLocation) (LocalVariables|GetLocalSpawnRotation) (LocalVariables|GetLocalSpawnScale)) "Undefined" 0 0))))
  (return _returnvalue _returnvalue_2))