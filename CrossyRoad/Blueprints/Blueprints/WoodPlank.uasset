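; WoodPlank is a moving plank actor in a Crossy Road-style game that slides along its local Y axis and removes itself when its lifetime runs out.
; SpawnAtLocation creates a new plank and sets its speed sign from the requested direction, with forward being negative Y.
; Tick moves it a fixed, frame-rate-dependent step and uses a Delay to count LifeTotal down about once per second until MovePlank destroys it at zero.
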(event EventTick
  (params (DeltaSeconds :type Float%20%28single-precision%29))
  (CallFunction|MovePlank)
  (Utilities|FlowControl|Delay 1.0)
  (CallFunction|DecrementLifeTotal))

(fn ConstructionScript)

(fn SpawnatLocation
  (params (SpawnLocation :type Vector) (WantsToMoveForward :type Boolean) (SpawnRotation :type Rotator))
  (bind _returnvalue (Game|SpawnActorfromClass "WoodPlank_C" (Math|Transform|MakeTransform SpawnLocation SpawnRotation "1,1,1") "Undefined" 0 0))
  (bind _output_get (Variables|WoodPlank_C|SetisMovingForward _returnvalue WantsToMoveForward))
  (if _output_get
    (Variables|WoodPlank_C|SetMoveSpeed _returnvalue -1e+01)
    (else
      (Variables|WoodPlank_C|SetMoveSpeed _returnvalue 1e+01)))
  (return _returnvalue))

(fn MovePlank
  (Class|Actor|AddActorLocalTransform (Math|Transform|MakeTransform (Math|Vector|MakeVector 0.0 (Variables|Default|GetMoveSpeed) 0.0) "0, 0, 0" "1,1,1") false false)
  (if (== 0 (Variables|Default|GetlifeTotal))
    (Actor|DestroyActor)))

(fn DecrementLifeTotal
  (Variables|Default|SetlifeTotal (- (Variables|Default|GetlifeTotal) 1)))