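; GrassRoad is a lane tile in a Crossy Road-style game that extends the level as the player advances.
; Either player trigger box spawns the next tile (GrassRoad at set score multiples, otherwise a Road with random 180-degree flip), adds points, then destroys this tile after a delay.
; A collision box recycles trucks, trains and police cars through their SpawnAtLocation at the obstacle spawn point.
; Initial obstacle spawning and wood plank logic are disconnected.
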(event OnComponentBeginOverlap(PlayerBox1)
  (params (OverlappedComponent :type Primitive%20Component%20Object%20Reference) (OtherActor :type Actor%20Object%20Reference) (OtherComp :type Primitive%20Component%20Object%20Reference) (OtherBodyIndex :type Integer) (bFromSweep :type Boolean) (SweepResult :type Hit%20Result%20Structure%20%28by%20ref%29))
  (bind _roadyspawnoffset (Variables|Default|GetRoadYSpawnOffset))
  (bind _staticmesh (Variables|Default|GetStaticMesh))
  (bind _defaultsceneroot (Variables|Default|GetDefaultSceneRoot))
  (bind _defaultsceneroot_2 (Variables|Default|GetDefaultSceneRoot))
  (bind _defaultsceneroot_3 (Variables|Default|GetDefaultSceneRoot))
  (bind _returnvalue (Transformation|GetWorldLocation _defaultsceneroot_2))
  (bind _returnvalue_2 (Transformation|GetWorldLocation _defaultsceneroot_3))
  (bind _returnvalue_3 (Transformation|GetWorldRotation _staticmesh))
  (bind _returnvalue_4 (Transformation|GetWorldScale _defaultsceneroot))
  (bind _returnvalue_5 (+ (.y _returnvalue) _roadyspawnoffset))
  ;[1 1 1] Player Box 1: Spawn / Despawn Road - 50% chance on rotation
  (Utilities|Casting|CastToCrossyRoadCharacter OtherActor)
  (if (not (Variables|Default|GetplayerAlreadyTriggeredBox))
    (Utilities|FlowControl|DoOnce false
      (:Completed
        (Variables|Default|SetplayerAlreadyTriggeredBox true)
        (bind _ascrossy_road_game_mode (Utilities|Casting|CastToCrossyRoadGameMode (Game|GetGameMode)))
        (if (== 0 (Math|Integer|%(Integer) (Variables|/Game/Blueprints/CrossyRoadGameMode.CrossyRoadGameMode_C|GetPlayerScore _ascrossy_road_game_mode) 11))
          (Game|SpawnActorfromClass "GrassRoad_C" (Math|Transform|MakeTransform (Math|Vector|MakeVector 0.0 (+ (Variables|Default|GetRoadYSpawnOffset) (.y _returnvalue_2)) (.z _returnvalue_2)) (Transformation|GetWorldRotation (Variables|Default|GetStaticMesh)) (Transformation|GetWorldScale (Variables|Default|GetDefaultSceneRoot))) "Undefined" 0 0)
          (elif (<= (Math|Random|RandomIntegerinRange 0 9) 4)
            (Game|SpawnActorfromClass "/Game/Blueprints/Road.Road_C" (Math|Transform|MakeTransform (Math|Vector|MakeVector 0.0 _returnvalue_5 (.z _returnvalue)) (Transformation|GetWorldRotation (Variables|Default|GetStaticMesh)) _returnvalue_4) "Undefined" 0 0)
            (Variables|Default|SetNewestWaterRoad 0)
            (else
              (Game|SpawnActorfromClass "/Game/Blueprints/Road.Road_C" (Math|Transform|MakeTransform (Math|Vector|MakeVector 7.56e+03 _returnvalue_5 (.z _returnvalue)) (Math|Rotator|MakeRotator (.roll _returnvalue_3) (.pitch _returnvalue_3) (+ (.yaw _returnvalue_3) 1.8e+02)) _returnvalue_4) "Undefined" 0 0)
              (Variables|Default|SetNewestWaterRoad 0))))
        (bind _ascrossy_road_game_mode_2 (Utilities|Casting|CastToCrossyRoadGameMode (Game|GetGameMode)))
        (Default|AddPlayerPoints _ascrossy_road_game_mode_2)
        (Utilities|FlowControl|Delay (Variables|Default|GetRoadLifeSpan))
        (Variables|Default|SetpendingDespawn true)
        (Actor|DestroyActor)))))

(event OnComponentBeginOverlap(TruckCollisionBox)
  (params (OverlappedComponent :type Primitive%20Component%20Object%20Reference) (OtherActor :type Actor%20Object%20Reference) (OtherComp :type Primitive%20Component%20Object%20Reference) (OtherBodyIndex :type Integer) (bFromSweep :type Boolean) (SweepResult :type Hit%20Result%20Structure%20%28by%20ref%29))
  (bind _staticmesh (Variables|Default|GetStaticMesh))
  (bind _staticmesh_2 (Variables|Default|GetStaticMesh))
  (bind _staticmesh_3 (Variables|Default|GetStaticMesh))
  (bind _returnvalue (Transformation|GetWorldRotation _staticmesh_2))
  (bind _returnvalue_2 (Transformation|GetWorldRotation _staticmesh))
  (bind _returnvalue_3 (Transformation|GetWorldRotation _staticmesh_3))
  ;[1 1 1] Obstical Collision
  ;;[0 0.03437 1] Despawn / Respawn Truck
  (bind _astruck (Utilities|Casting|CastToTruck OtherActor)
    (:then
      (bind _output_get (Variables|Default|SetNewestTruck _astruck))
      (Variables|/Game/Blueprints/Truck.Truck_C|SethasTriggeredBox _astruck true)
      (Default|SpawnatLocation _output_get (Transformation|GetWorldLocation (Variables|Default|GetObsticalSpawnLocation)) true (Math|Rotator|MakeRotator (.roll _returnvalue_3) (* (.pitch _returnvalue_3) -1.0) (.yaw _returnvalue_3)))
      (Actor|DestroyActor _astruck))
    (:CastFailed
      ;;[1 0.9943 0.01025] Despawn / Respawn Train
      (bind _astrain (Utilities|Casting|CastToTrain OtherActor)
        (:then
          (bind _output_get_2 (Variables|Default|SetNewestTrain _astrain))
          (Variables|/Game/Blueprints/Train.Train_C|SethasTriggeredBox _astrain true)
          (Default|SpawnatLocation _output_get_2 (Transformation|GetWorldLocation (Variables|Default|GetObsticalSpawnLocation)) false (Math|Rotator|MakeRotator (.roll _returnvalue) (* (.pitch _returnvalue) -1.0) (.yaw _returnvalue)))
          (Actor|DestroyActor _astrain))
        (:CastFailed
          ;;[0.1666 1 0.9901] Despawn / Respawn Police Car
          (bind _aspolice_car (Utilities|Casting|CastToPoliceCar OtherActor))
          (bind _output_get_3 (Variables|Default|SetNewestPoliceCar _aspolice_car))
          (Variables|/Game/Blueprints/PoliceCar.PoliceCar_C|SethasTriggeredBox _aspolice_car false)
          (Default|SpawnatLocation _output_get_3 (Transformation|GetWorldLocation (Variables|Default|GetObsticalSpawnLocation)) false (Math|Rotator|MakeRotator (.roll _returnvalue_2) (* (.pitch _returnvalue_2) -1.0) (.yaw _returnvalue_2)))
          (Actor|DestroyActor _aspolice_car))))))

(event OnComponentBeginOverlap(PlayerBox2)
  (params (OverlappedComponent :type Primitive%20Component%20Object%20Reference) (OtherActor :type Actor%20Object%20Reference) (OtherComp :type Primitive%20Component%20Object%20Reference) (OtherBodyIndex :type Integer) (bFromSweep :type Boolean) (SweepResult :type Hit%20Result%20Structure%20%28by%20ref%29))
  (bind _defaultsceneroot (Variables|Default|GetDefaultSceneRoot))
  (bind _defaultsceneroot_2 (Variables|Default|GetDefaultSceneRoot))
  (bind _defaultsceneroot_3 (Variables|Default|GetDefaultSceneRoot))
  (bind _staticmesh (Variables|Default|GetStaticMesh))
  (bind _defaultsceneroot_4 (Variables|Default|GetDefaultSceneRoot))
  (bind _returnvalue (Transformation|GetWorldLocation _defaultsceneroot))
  (bind _returnvalue_2 (Transformation|GetWorldScale _defaultsceneroot_2))
  (bind _returnvalue_3 (Transformation|GetWorldLocation _defaultsceneroot_3))
  (bind _returnvalue_4 (Transformation|GetWorldRotation _staticmesh))
  (bind _returnvalue_5 (Transformation|GetWorldLocation _defaultsceneroot_4))
  ;[1 1 1] PlayerBox 2: Spawn / Despawn Road - 50% chance on rotation
  (Utilities|Casting|CastToCrossyRoadCharacter OtherActor)
  (if (not (Variables|Default|GetplayerAlreadyTriggeredBox))
    (Utilities|FlowControl|DoOnce false
      (:Completed
        (Variables|Default|SetplayerAlreadyTriggeredBox true)
        (bind _ascrossy_road_game_mode (Utilities|Casting|CastToCrossyRoadGameMode (Game|GetGameMode)))
        (if (== 0 (Math|Integer|%(Integer) (Variables|/Game/Blueprints/CrossyRoadGameMode.CrossyRoadGameMode_C|GetPlayerScore _ascrossy_road_game_mode) 5))
          (Game|SpawnActorfromClass "GrassRoad_C" (Math|Transform|MakeTransform (Math|Vector|MakeVector 0.0 (+ (Variables|Default|GetRoadYSpawnOffset) (.y _returnvalue_5)) (.z _returnvalue_5)) (Transformation|GetWorldRotation (Variables|Default|GetStaticMesh)) (Transformation|GetWorldScale (Variables|Default|GetDefaultSceneRoot))) "Undefined" 0 0)
          (elif (<= (Math|Random|RandomIntegerinRange 0 9) 4)
            (Game|SpawnActorfromClass "/Game/Blueprints/Road.Road_C" (Math|Transform|MakeTransform (Math|Vector|MakeVector 7.56e+03 (+ (.y _returnvalue) (Variables|Default|GetRoadYSpawnOffset)) (.z _returnvalue)) (Transformation|GetWorldRotation (Variables|Default|GetStaticMesh)) _returnvalue_2) "Undefined" 0 0)
            (Variables|Default|SetNewestRoad 0)
            (else
              (Game|SpawnActorfromClass "/Game/Blueprints/Road.Road_C" (Math|Transform|MakeTransform (Math|Vector|MakeVector 0.0 (+ (.y _returnvalue_3) (Variables|Default|GetRoadYSpawnOffset)) (.z _returnvalue_3)) (Math|Rotator|MakeRotator (.roll _returnvalue_4) (.pitch _returnvalue_4) (+ (.yaw _returnvalue_4) 1.8e+02)) _returnvalue_2) "Undefined" 0 0)
              (Variables|Default|SetNewestRoad 0))))
        (bind _ascrossy_road_game_mode_2 (Utilities|Casting|CastToCrossyRoadGameMode (Game|GetGameMode)))
        (Default|AddPlayerPoints _ascrossy_road_game_mode_2)
        (Utilities|FlowControl|Delay (Variables|Default|GetRoadLifeSpan))
        (Actor|DestroyActor)))))

(event EventBeginPlay
  ;[1 1 1] Comment
)

(fn ConstructionScript)

(fn SpawnRoadatLocation
  (params (SpawnLocation :type Vector))
  (Game|SpawnActorfromClass "/Game/Blueprints/Road.Road_C" (Math|Transform|MakeTransform SpawnLocation "0, 0, 0" "1,1,1") "Undefined" 0 0))