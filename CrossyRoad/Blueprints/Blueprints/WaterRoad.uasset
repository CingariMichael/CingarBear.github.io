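; WaterRoad is a Crossy Road water lane that spawns a WoodPlank on BeginPlay and recycles planks reaching TruckCollisionBox.
; Two player boxes spawn the next lane on crossing: GrassRoad when score is divisible by 11, otherwise usually WaterRoad with randomly flipped yaw.
; They then add points and destroy this road after RoadLifeSpan.
; PlayerDespawnBox, meant to despawn players hitting water, sets the character's WasHit to false.
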(event OnComponentBeginOverlap(PlayerBox1)
  (params (OverlappedComponent :type Primitive%20Component%20Object%20Reference) (OtherActor :type Actor%20Object%20Reference) (OtherComp :type Primitive%20Component%20Object%20Reference) (OtherBodyIndex :type Integer) (bFromSweep :type Boolean) (SweepResult :type Hit%20Result%20Structure%20%28by%20ref%29))
  (bind _staticmesh (Variables|Components|GetStaticMesh))
  (bind _defaultsceneroot (Variables|Components|GetDefaultSceneRoot))
  (bind _roadspawnoffset (Variables|Default|GetRoadSpawnOffset))
  (bind _defaultsceneroot_2 (Variables|Components|GetDefaultSceneRoot))
  (bind _defaultsceneroot_3 (Variables|Components|GetDefaultSceneRoot))
  (bind _returnvalue (Transformation|GetWorldScale _defaultsceneroot_2))
  (bind _returnvalue_2 (Transformation|GetWorldRotation _staticmesh))
  (bind _returnvalue_3 (Transformation|GetWorldLocation _defaultsceneroot))
  (bind _returnvalue_4 (Transformation|GetWorldLocation _defaultsceneroot_3))
  (bind _returnvalue_5 (+ _roadspawnoffset (.y _returnvalue_3)))
  ;[1 1 1] PlayerBox 1
  ;;[0.5529 0 0] Check if Player collides with Playerbox 1
  (Utilities|Casting|CastToCrossyRoadCharacter OtherActor)
  (if (not (Variables|Default|GetplayerAlreadyTriggeredBox))
    (Utilities|FlowControl|DoOnce false
      (:Completed
        (Variables|Default|SetplayerAlreadyTriggeredBox true)
        ;;[0 1 0.07942] Spawn a Grass Road based on player score
        (bind _ascrossy_road_game_mode (Utilities|Casting|CastToCrossyRoadGameMode (Game|GetGameMode)))
        (if (== 0 (Math|Integer|%(Integer) (Variables|/Game/Blueprints/CrossyRoadGameMode.CrossyRoadGameMode_C|GetPlayerScore _ascrossy_road_game_mode) 11))
          (Game|SpawnActorfromClass "/Game/Blueprints/GrassRoad.GrassRoad_C" (Math|Transform|MakeTransform (Math|Vector|MakeVector 0.0 (+ (Variables|Default|GetRoadSpawnOffset) (.y _returnvalue_4)) (.z _returnvalue_4)) (Transformation|GetWorldRotation (Variables|Components|GetStaticMesh)) (Transformation|GetWorldScale (Variables|Components|GetDefaultSceneRoot))) "Undefined" 0 0)
          (else
            ;;[0 0.9725 1] Spawn new Water Road with random rotation
            (if (<= (Math|Random|RandomIntegerinRange 0 9) 4)
              (Game|SpawnActorfromClass "WaterRoad_C" (Math|Transform|MakeTransform (Math|Vector|MakeVector 0.0 _returnvalue_5 (.z _returnvalue_3)) (Transformation|GetWorldRotation (Variables|Components|GetStaticMesh)) _returnvalue) "Undefined" 0 0)
              (Variables|Default|SetNewestRoad 0)
              (else
                (Game|SpawnActorfromClass "WaterRoad_C" (Math|Transform|MakeTransform (Math|Vector|MakeVector 7.56e+03 _returnvalue_5 (.z _returnvalue_3)) (Math|Rotator|MakeRotator (.roll _returnvalue_2) (.pitch _returnvalue_2) (+ (.yaw _returnvalue_2) 1.8e+02)) _returnvalue) "Undefined" 0 0)
                (Variables|Default|SetNewestRoad 0)))))
        ;;[0.5529 0 0] Increment Player Score and Despawn crossed road
        (bind _ascrossy_road_game_mode_2 (Utilities|Casting|CastToCrossyRoadGameMode (Game|GetGameMode)))
        (Default|AddPlayerPoints _ascrossy_road_game_mode_2)
        (Utilities|FlowControl|Delay (Variables|Default|GetRoadLifeSpan))
        (Variables|Default|SetpendingDespawn true)
        (Actor|DestroyActor)))))

(event OnComponentBeginOverlap(TruckCollisionBox)
  (params (OverlappedComponent :type Primitive%20Component%20Object%20Reference) (OtherActor :type Actor%20Object%20Reference) (OtherComp :type Primitive%20Component%20Object%20Reference) (OtherBodyIndex :type Integer) (bFromSweep :type Boolean) (SweepResult :type Hit%20Result%20Structure%20%28by%20ref%29))
  ;[0.2863 0.09804 0] Trigger - Despawn WoodPlank obstical and spawn a new one
  (bind _aswood_plank (Utilities|Casting|CastToWoodPlank OtherActor))
  (bind _output_get (Variables|Default|SetNewestObstical _aswood_plank))
  (Variables|/Game/Blueprints/WoodPlank.WoodPlank_C|SethasTriggeredBox _aswood_plank false)
  (Default|SpawnatLocation _output_get (Transformation|GetWorldLocation (Variables|Components|GetObsticalSpawnLocation)) false (Transformation|GetWorldRotation (Variables|Components|GetStaticMesh)))
  (Actor|DestroyActor _aswood_plank))

(event OnComponentBeginOverlap(PlayerBox2)
  (params (OverlappedComponent :type Primitive%20Component%20Object%20Reference) (OtherActor :type Actor%20Object%20Reference) (OtherComp :type Primitive%20Component%20Object%20Reference) (OtherBodyIndex :type Integer) (bFromSweep :type Boolean) (SweepResult :type Hit%20Result%20Structure%20%28by%20ref%29))
  (bind _defaultsceneroot (Variables|Components|GetDefaultSceneRoot))
  (bind _defaultsceneroot_2 (Variables|Components|GetDefaultSceneRoot))
  (bind _roadspawnoffset (Variables|Default|GetRoadSpawnOffset))
  (bind _staticmesh (Variables|Components|GetStaticMesh))
  (bind _defaultsceneroot_3 (Variables|Components|GetDefaultSceneRoot))
  (bind _returnvalue (Transformation|GetWorldLocation _defaultsceneroot))
  (bind _returnvalue_2 (Transformation|GetWorldScale _defaultsceneroot_2))
  (bind _returnvalue_3 (Transformation|GetWorldRotation _staticmesh))
  (bind _returnvalue_4 (Transformation|GetWorldLocation _defaultsceneroot_3))
  (bind _returnvalue_5 (+ _roadspawnoffset (.y _returnvalue)))
  ;[1 1 1] Playerbox 2
  ;;[0.5529 0 0] Check if Player Collides with Playerbox 2
  (Utilities|Casting|CastToCrossyRoadCharacter OtherActor)
  (if (not (Variables|Default|GetplayerAlreadyTriggeredBox))
    (Utilities|FlowControl|DoOnce false
      (:Completed
        (Variables|Default|SetplayerAlreadyTriggeredBox true)
        ;;[0 1 0.07942] Spawn a Grass Road based on player score
        (bind _ascrossy_road_game_mode (Utilities|Casting|CastToCrossyRoadGameMode (Game|GetGameMode)))
        (if (== 0 (Math|Integer|%(Integer) (Variables|/Game/Blueprints/CrossyRoadGameMode.CrossyRoadGameMode_C|GetPlayerScore _ascrossy_road_game_mode) 11))
          (Game|SpawnActorfromClass "/Game/Blueprints/GrassRoad.GrassRoad_C" (Math|Transform|MakeTransform (Math|Vector|MakeVector 0.0 (+ (Variables|Default|GetRoadSpawnOffset) (.y _returnvalue_4)) (.z _returnvalue_4)) (Transformation|GetWorldRotation (Variables|Components|GetStaticMesh)) (Transformation|GetWorldScale (Variables|Components|GetDefaultSceneRoot))) "Undefined" 0 0)
          (else
            ;;[0 0.9725 1] Spawn new water road a with random rotation
            (if (<= (Math|Random|RandomIntegerinRange 0 9) 4)
              (Game|SpawnActorfromClass "WaterRoad_C" (Math|Transform|MakeTransform (Math|Vector|MakeVector 7.56e+03 _returnvalue_5 (.z _returnvalue)) (Transformation|GetWorldRotation (Variables|Components|GetStaticMesh)) _returnvalue_2) "Undefined" 0 0)
              (Variables|Default|SetNewestRoad 0)
              (else
                (Game|SpawnActorfromClass "WaterRoad_C" (Math|Transform|MakeTransform (Math|Vector|MakeVector 0.0 _returnvalue_5 (.z _returnvalue)) (Math|Rotator|MakeRotator (.roll _returnvalue_3) (.pitch _returnvalue_3) (+ (.yaw _returnvalue_3) 1.8e+02)) _returnvalue_2) "Undefined" 0 0)
                (Variables|Default|SetNewestRoad 0)))))
        ;;[0.5529 0 0] Increment player's score and despawn crossed road
        (bind _ascrossy_road_game_mode_2 (Utilities|Casting|CastToCrossyRoadGameMode (Game|GetGameMode)))
        (Default|AddPlayerPoints _ascrossy_road_game_mode_2)
        (Utilities|FlowControl|Delay (Variables|Default|GetRoadLifeSpan))
        (Actor|DestroyActor)))))

(event OnComponentBeginOverlap(PlayerDespawnBox)
  (params (OverlappedComponent :type Primitive%20Component%20Object%20Reference) (OtherActor :type Actor%20Object%20Reference) (OtherComp :type Primitive%20Component%20Object%20Reference) (OtherBodyIndex :type Integer) (bFromSweep :type Boolean) (SweepResult :type Hit%20Result%20Structure%20%28by%20ref%29))
  ;[1 1 1] PlayerBox 1
  ;;[0 0.9725 1] Despawn the Player if it hits the water
  (bind _ascrossy_road_character (Utilities|Casting|CastToCrossyRoadCharacter OtherActor))
  (Variables|/Game/Blueprints/CrossyRoadCharacter.CrossyRoadCharacter_C|SetwasHit _ascrossy_road_character false))

(event EventBeginPlay
  (bind _staticmesh (Variables|Components|GetStaticMesh))
  (bind _returnvalue (Transformation|GetWorldRotation _staticmesh))
  ;[0.2863 0.09804 0] Spawn WoodPlank obstical when a WaterRoad is spawned
  (Game|SpawnActorfromClass "/Game/Blueprints/WoodPlank.WoodPlank_C" (Math|Transform|MakeTransform (Transformation|GetWorldLocation (Variables|Components|GetObsticalSpawnLocation)) (Math|Rotator|MakeRotator (.roll _returnvalue) (* (.pitch _returnvalue) -1.0) (.yaw _returnvalue)) "1,1,1") "Undefined" 0 0)
  (Variables|Default|SetRoadzRotation (.yaw (Transformation|GetWorldRotation (Variables|Components|GetDefaultSceneRoot)))))

(fn ConstructionScript)

(fn SpawnRoadatLocation
  (params (SpawnLocation :type Vector))
  (Game|SpawnActorfromClass "/Game/Blueprints/Road.Road_C" (Math|Transform|MakeTransform SpawnLocation "0, 0, 0" "1,1,1") "Undefined" 0 0))