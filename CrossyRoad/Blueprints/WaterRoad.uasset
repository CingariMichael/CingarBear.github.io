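; WaterRoad is an endless-runner water lane for a Crossy Road-style game, carrying WoodPlank obstacles.
; It spawns a plank on BeginPlay, then respawns it at the start point whenever one hits the end trigger.
; Either player trigger spawns another WaterRoad, randomly normal or flipped 180 degrees, and awards points through the game mode.
; The crossed lane destroys itself after a lifespan delay.
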(event OnComponentBeginOverlap(PlayerBox1)
  (params (OverlappedComponent :type Primitive%20Component%20Object%20Reference) (OtherActor :type Actor%20Object%20Reference) (OtherComp :type Primitive%20Component%20Object%20Reference) (OtherBodyIndex :type Integer) (bFromSweep :type Boolean) (SweepResult :type Hit%20Result%20Structure%20%28by%20ref%29))
  (bind _staticmesh (Variables|Default|GetStaticMesh))
  (bind _returnvalue (Transformation|GetWorldRotation _staticmesh))
  ;[1 1 1] Trigger - Spawn road when player crosses road - Facing East (towards negative X)
  (Utilities|Casting|CastToCrossyRoadCharacter OtherActor)
  (if (not (Variables|Default|GetplayerAlreadyTriggeredBox))
    (Utilities|FlowControl|DoOnce false
      (:Completed
        (Variables|Default|SetplayerAlreadyTriggeredBox true)
        (if (<= (Math|Random|RandomIntegerinRange 0 9) 4)
          (Game|SpawnActorfromClass "WaterRoad_C" (Math|Transform|MakeTransform (Transformation|GetWorldLocation (Variables|Default|GetNewRoadSpawnLocation%20%28PlayerBox1%29)) (Transformation|GetWorldRotation (Variables|Default|GetStaticMesh)) "1,1,1") "Undefined" 0 0)
          (Variables|Default|SetNewestRoad 0)
          (else
            (Game|SpawnActorfromClass "WaterRoad_C" (Math|Transform|MakeTransform (Transformation|GetWorldLocation (Variables|Default|GetFlippedRoadSpawnLocation%20%28PlayerBox1%29)) (Math|Rotator|MakeRotator (.roll _returnvalue) (.pitch _returnvalue) (+ (.yaw _returnvalue) 1.8e+02)) "1,1,1") "Undefined" 0 0)
            (Variables|Default|SetNewestRoad 0)))
        (bind _ascrossy_road_game_mode (Utilities|Casting|CastToCrossyRoadGameMode (Game|GetGameMode)))
        (Default|AddPlayerPoints _ascrossy_road_game_mode)
        (Utilities|FlowControl|Delay (Variables|Default|GetRoadLifeSpan))
        (Variables|Default|SetpendingDespawn true)
        (Actor|DestroyActor)))))

(event OnComponentBeginOverlap(TruckCollisionBox)
  (params (OverlappedComponent :type Primitive%20Component%20Object%20Reference) (OtherActor :type Actor%20Object%20Reference) (OtherComp :type Primitive%20Component%20Object%20Reference) (OtherBodyIndex :type Integer) (bFromSweep :type Boolean) (SweepResult :type Hit%20Result%20Structure%20%28by%20ref%29))
  ;[1 1 1] Trigger - Respawn Truck obstical and despawn old Truck obstical
  (bind _aswood_plank (Utilities|Casting|CastToWoodPlank OtherActor))
  (bind _output_get (Variables|Default|SetNewestObstical _aswood_plank))
  (Variables|/Game/Blueprints/WoodPlank.WoodPlank_C|SethasTriggeredBox _aswood_plank false)
  (Default|SpawnatLocation _output_get (Transformation|GetWorldLocation (Variables|Default|GetObsticalSpawnLocation)) false (Transformation|GetWorldRotation (Variables|Default|GetStaticMesh)))
  (Actor|DestroyActor _aswood_plank))

(event OnComponentBeginOverlap(PlayerBox2)
  (params (OverlappedComponent :type Primitive%20Component%20Object%20Reference) (OtherActor :type Actor%20Object%20Reference) (OtherComp :type Primitive%20Component%20Object%20Reference) (OtherBodyIndex :type Integer) (bFromSweep :type Boolean) (SweepResult :type Hit%20Result%20Structure%20%28by%20ref%29))
  (bind _staticmesh (Variables|Default|GetStaticMesh))
  (bind _defaultsceneroot (Variables|Default|GetDefaultSceneRoot))
  (bind _returnvalue (Transformation|GetWorldScale _defaultsceneroot))
  (bind _returnvalue_2 (Transformation|GetWorldRotation _staticmesh))
  ;[1 1 1] Trigger - Spawn road when player crosses road - Facing West (towards positive X)
  (Utilities|Casting|CastToCrossyRoadCharacter OtherActor)
  (if (not (Variables|Default|GetplayerAlreadyTriggeredBox))
    (Utilities|FlowControl|DoOnce false
      (:Completed
        (Variables|Default|SetplayerAlreadyTriggeredBox true)
        (if (<= (Math|Random|RandomIntegerinRange 0 9) 4)
          (Game|SpawnActorfromClass "WaterRoad_C" (Math|Transform|MakeTransform (Transformation|GetWorldLocation (Variables|Default|GetNewRoadSpawnLocation%20%28PlayerBox2%29)) (Transformation|GetWorldRotation (Variables|Default|GetStaticMesh)) _returnvalue) "Undefined" 0 0)
          (Variables|Default|SetNewestRoad 0)
          (else
            (Game|SpawnActorfromClass "WaterRoad_C" (Math|Transform|MakeTransform (Transformation|GetWorldLocation (Variables|Default|GetFlippedRoadSpawnLocation%20%28PlayerBox2%29)) (Math|Rotator|MakeRotator (.roll _returnvalue_2) (.pitch _returnvalue_2) (+ (.yaw _returnvalue_2) 1.8e+02)) _returnvalue) "Undefined" 0 0)
            (Variables|Default|SetNewestRoad 0)))
        (bind _ascrossy_road_game_mode (Utilities|Casting|CastToCrossyRoadGameMode (Game|GetGameMode)))
        (Default|AddPlayerPoints _ascrossy_road_game_mode)
        (Utilities|FlowControl|Delay (Variables|Default|GetRoadLifeSpan))
        (Actor|DestroyActor)))))

(event EventBeginPlay
  (bind _staticmesh (Variables|Default|GetStaticMesh))
  (bind _returnvalue (Transformation|GetWorldRotation _staticmesh))
  (Game|SpawnActorfromClass "/Game/Blueprints/WoodPlank.WoodPlank_C" (Math|Transform|MakeTransform (Transformation|GetWorldLocation (Variables|Default|GetObsticalSpawnLocation)) (Math|Rotator|MakeRotator (.roll _returnvalue) (* (.pitch _returnvalue) -1.0) (.yaw _returnvalue)) "1,1,1") "Undefined" 0 0))

(fn ConstructionScript)

(fn SpawnRoadatLocation
  (params (SpawnLocation :type Vector))
  (Game|SpawnActorfromClass "/Game/Blueprints/Road.Road_C" (Math|Transform|MakeTransform SpawnLocation "0, 0, 0" "1,1,1") "Undefined" 0 0))